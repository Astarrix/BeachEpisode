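; BP_Card_HolyBullets is a card ability, a child in the card master family, that gives the player pawn a damage bonus while active.
; ActivateAbility raises the pawn's DamageMultiplier by half, and EndAbility reverses this by scaling it to two-thirds, so the change is relative to the current value.
; Both print a debug message, then call the parent implementation.
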(fn ConstructionScript
  (|CallParentFunction))

(fn ActivateAbility
  (bind _player_pawn (Variables|Default|GetPlayer%20Pawn))
  (Variables|/Game/Player/BP_Character_Player.BP_Character_Player_C|SetDamageMultiplier _player_pawn (* (Variables|/Game/Player/BP_Character_Player.BP_Character_Player_C|GetDamageMultiplier _player_pawn) 1.5))
  (Development|PrintString "Damage Bonus Applied" true true "(R=1.000000,G=0.000000,B=0.000000,A=1.000000)")
  (|CallParentFunction))

(fn EndAbility
  (bind _player_pawn (Variables|Default|GetPlayer%20Pawn))
  (Variables|/Game/Player/BP_Character_Player.BP_Character_Player_C|SetDamageMultiplier _player_pawn (* (/ (Variables|/Game/Player/BP_Character_Player.BP_Character_Player_C|GetDamageMultiplier _player_pawn) 3.0) 2.0))
  (Development|PrintString "Damage Bonus Removed" true true "(R=1.000000,G=0.000000,B=0.000000,A=1.000000)")
  (|CallParentFunction))