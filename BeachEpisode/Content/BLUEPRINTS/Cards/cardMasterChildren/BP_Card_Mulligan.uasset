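; BP_Card_Mulligan is a card ability, a child of the card master, that triggers a mulligan of the player's hand.
; EndAbility hands the work to Mulligan on the player pawn's BPCCardManager and does not call the parent EndAbility.
; A disconnected older graph does it inline: it discards every occupied HandIDs slot, begins that many new cards, then calls the parent EndAbility.
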(fn ConstructionScript
  (|CallParentFunction))

(fn EndAbility
  (Default|Mulligan (Variables|/Game/Player/BP_Character_Player.BP_Character_Player_C|GetBPC_CardManager (Variables|Default|GetPlayer%20Pawn))))