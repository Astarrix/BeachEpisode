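; Player component that runs a real-time card hand: four input slots spawn each card's actor on the floor ahead via two line traces.
; Timed draws refill empty slots from a shuffled deck of DT_Cards IDs, reshuffling discards when it empties, and update the HUD card holder.
; A hand totalling 21 (aces 1 or 11) starts a timed Blackjack state with its own draw delay, then redraws the held cards.
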(event Custom|AddNewCardUI
  (params (Position :type Integer) (ID :type Integer))
  ;[0.05098 0.05098 0.05098] AddNewCardUI
  (bind _outrownames (DataTable|GetDataTableRowNames "/Game/BLUEPRINTS/Cards/DT_Cards.DT_Cards"))
  (bind _returnvalue (Utilities|GetDataTableRow "/Game/BLUEPRINTS/Cards/DT_Cards.DT_Cards" (Utilities|Array|Get(acopy) _outrownames (- ID 1)))
    (:then
      (Default|NewCard (Variables|References|GetUI%20Card%20Holder) Position _returnvalue)
      (if (.isBlackjack (CallFunction|CheckforBlackjack))
        (CallFunction|BeginBlackjackTimer)))))

(event Custom|AddMappingContext
  ;[0.05098 0.05098 0.05098] Add Mapping Context
  (Input|AddMappingContext (PlayerController|LocalPlayerSubsystems|GetEnhancedInputLocalPlayerSubsystem (Variables|/Game/Player/Character_Player.Character_Player_C|GetOwningController (Variables|References|GetAs%20PLAYER))) "/Game/Systems/Inputs/IMC_Cards.IMC_Cards" 0 "(bIgnoreAllPressedKeysUntilRelease=True,bForceImmediately=False)"))

(event Custom|SpawnCardActor
  (params (ID :type Integer))
  ;[0.05098 0.05098 0.05098] SpawnCardActor
  (bind (_isvalidid _outcardinfo) (CallFunction|GetDatafromID ID))
  (if _isvalidid
    (bind _returnvalue (Game|SpawnActorfromClass (.AssignedActor (Utilities|Struct|BreaksCardInfo _outcardinfo)) (CallFunction|GetCardSpawnTransform 4e+02) "AdjustIfPossibleButAlwaysSpawn" "MultiplyWithRoot" 0 (Variables|References|GetAs%20PLAYER) 0))
    (Default|Initialise _returnvalue _outcardinfo)))

(event Custom|BeginNewCard
  (bind _handids (Variables|Default|GetHandIDs))
  ;[0 1 0] Checks for empty card slot and draws a card into it. Removes that card from the deck list
  (bind (_array_element _array_index) (Utilities|Array|ForEachLoopwithBreak (Variables|Default|GetHandIDs) :!label _label)
    (:LoopBody
      (if (== _array_element -1)
        (Utilities|Array|SetArrayElem _handids _array_index (Utilities|Array|Get(acopy) (Variables|Default|GetdeckIDs)))
        (Utilities|Array|RemoveIndex (Variables|Default|GetdeckIDs))
        (CallFunction|AddNewCardUI _array_index (Utilities|Array|Get(acopy) _handids _array_index))
        (goto _label Break)))
    (:Completed
      (CallFunction|CheckforEmptyDeck))))

(event Custom|CheckForEmptyDeck
  (bind _discardpileids (Variables|Default|GetdiscardPileIDs))
  ;[0 1 0] Checks for an empty deck. If empty, shuffles discard into new deck
  (if (== (Utilities|Array|Length (Variables|Default|GetdeckIDs)) 0)
    (Utilities|Array|Shuffle _discardpileids)
    (Variables|Default|SetdeckIDs _discardpileids)
    (Utilities|Array|Clear _discardpileids)))

(event Custom|Discard%20Card
  (params (hand%20Index :type Integer))
  ;[0 1 0] Discards a card at given hand index (without triggering effect)
  (Utilities|Array|Add (Variables|Default|GetdiscardPileIDs) (Utilities|Array|Get(acopy) (Variables|Default|GetHandIDs) hand%20Index))
  (Utilities|Array|SetArrayElem (Variables|Default|GetHandIDs) hand%20Index -1)
  (Default|UseCardUI (Variables|References|GetUI%20Card%20Holder) hand%20Index))

(event Custom|Mulligan
  (bind _cards_discarded (CallFunction|DiscardHand))
  (for _index (range 1 _cards_discarded)
    (CallFunction|BeginNewCard)))

(event Custom|AttemptDrawTimer
  ;[0.05098 0.05098 0.05098] Timer
  (if (Utilities|Array|ContainsItem (Variables|Default|GetHandIDs) -1) ; checks if there are any slots still open
    (if (Utilities|Time|IsValidTimerHandle (Variables|Default|GetCardDrawTimerHandle)) ; checks if the timer is running, if not begins it
      (if (Utilities|Time|IsValidTimerHandle (Variables|Blackjack|GetBlackjackTimerHandle))
        (Utilities|Time|ClearandInvalidateTimerbyHandle (Variables|Default|GetCardDrawTimerHandle))
        (CallFunction|AttemptDrawTimer))
      (else
        (bind _returnvalue (Utilities|Time|SetTimerbyEvent (delegate Custom|DrawTimerFinished) (CallFunction|GetCardDrawTime)))
        (Variables|Default|SetCardDrawTimerHandle _returnvalue)
        (Default|BeginNewCardTimer (Variables|References|GetUI%20Card%20Holder) (CallFunction|GetCardDrawTime))))
    (else
      (Utilities|Time|ClearandInvalidateTimerbyHandle (Variables|Default|GetCardDrawTimerHandle)))))

(event Custom|DrawTimerFinished
  ;[0.05098 0.05098 0.05098] Timer
  (CallFunction|BeginNewCard)
  (Utilities|Time|ClearandInvalidateTimerbyHandle (Variables|Default|GetCardDrawTimerHandle))
  (CallFunction|AttemptDrawTimer) ; if multiple cards have been used, this keeps the thing going
)

(event Custom|LoadDeck
  ;[0 1 0] Add code to load deck to deckIDs from instance
  (Utilities|Array|Shuffle (Variables|Default|GetdeckIDs)))

(event Custom|BeginBlackjackTimer
  ;[0.05098 0.05098 0.05098] BlackjackTimer
  (bind _returnvalue (Utilities|Time|SetTimerbyEvent (delegate Custom|EndBlackjack) (Variables|Blackjack|GetBlackjackDuration)))
  (Variables|Blackjack|SetBlackjackTimerHandle _returnvalue)
  (CallFunction|AttemptDrawTimer)
  (Default|BlackjackUIToggle (Variables|References|GetUI%20Card%20Holder) (Utilities|Time|IsValidTimerHandle (Variables|Blackjack|GetBlackjackTimerHandle)) (Variables|Blackjack|GetBlackjackDuration)))

(event Custom|EndBlackjack
  (bind _blackjacktimerhandle (Variables|Blackjack|GetBlackjackTimerHandle))
  ;[0.05098 0.05098 0.05098] BlackjackTimer
  (Utilities|Time|ClearandInvalidateTimerbyHandle _blackjacktimerhandle)
  (CallFunction|Mulligan)
  (Default|BlackjackUIToggle (Variables|References|GetUI%20Card%20Holder) (Utilities|Time|IsValidTimerHandle _blackjacktimerhandle) (Variables|Blackjack|GetBlackjackDuration)))

(event Custom|UseCardUI
  (params (Position :type Integer))
  ;[0.05098 0.05098 0.05098] UseCardUI
  (Default|UseCardUI (Variables|References|GetUI%20Card%20Holder) Position)
  (CallFunction|AttemptDrawTimer)
  (if (.isBlackjack (CallFunction|CheckforBlackjack))
    (CallFunction|BeginBlackjackTimer)))

(event Custom|LoadAllCards
  ;[0.05098 0.05098 0.05098] When game starts, fill the hand
  (for _array_element (Variables|Default|GetHandIDs)
    (CallFunction|BeginNewCard)))

(event Input|EnhancedActionEvents|EnhancedInputActionIA_CardSlot1
  (params (ActionValue :type Boolean) (ElapsedSeconds :type Float%20%28double-precision%29) (TriggeredSeconds :type Float%20%28double-precision%29) (InputAction :type Input%20Action%20Object%20Reference :default "/Game/Systems/Inputs/Actions/Cards/IA_CardSlot1.IA_CardSlot1"))
  ;[0.05098 0.05098 0.05098] TriggerEvents
  (:Started
    (bind _success (CallFunction|UseCard))
    (if _success
      (CallFunction|UseCardUI)
      (else
        (Development|PrintString "CARD 1 FAILED USE")))))

(event Input|EnhancedActionEvents|EnhancedInputActionIA_CardSlot2
  (params (ActionValue :type Boolean) (ElapsedSeconds :type Float%20%28double-precision%29) (TriggeredSeconds :type Float%20%28double-precision%29) (InputAction :type Input%20Action%20Object%20Reference :default "/Game/Systems/Inputs/Actions/Cards/IA_CardSlot2.IA_CardSlot2"))
  ;[0.05098 0.05098 0.05098] TriggerEvents
  (:Started
    (bind _success (CallFunction|UseCard 1))
    (if _success
      (CallFunction|UseCardUI 1)
      (else
        (Development|PrintString "CARD 2 FAILED USE")))))

(event Input|EnhancedActionEvents|EnhancedInputActionIA_CardSlot3
  (params (ActionValue :type Boolean) (ElapsedSeconds :type Float%20%28double-precision%29) (TriggeredSeconds :type Float%20%28double-precision%29) (InputAction :type Input%20Action%20Object%20Reference :default "/Game/Systems/Inputs/Actions/Cards/IA_CardSlot3.IA_CardSlot3"))
  ;[0.05098 0.05098 0.05098] TriggerEvents
  (:Started
    (bind _success (CallFunction|UseCard 2))
    (if _success
      (CallFunction|UseCardUI 2)
      (else
        (Development|PrintString "CARD 3 FAILED USE")))))

(event Input|EnhancedActionEvents|EnhancedInputActionIA_CardSlot4
  (params (ActionValue :type Boolean) (ElapsedSeconds :type Float%20%28double-precision%29) (TriggeredSeconds :type Float%20%28double-precision%29) (InputAction :type Input%20Action%20Object%20Reference :default "/Game/Systems/Inputs/Actions/Cards/IA_CardSlot4.IA_CardSlot4"))
  ;[0.05098 0.05098 0.05098] TriggerEvents
  (:Started
    (bind _success (CallFunction|UseCard 3))
    (if _success
      (CallFunction|UseCardUI 3)
      (else
        (Development|PrintString "CARD 4 FAILED USE")))))

(event EventBeginPlay
  ;[0.05098 0.05098 0.05098] BeginPlay&SaveVariables
  (bind _ascharacter_player (Utilities|Casting|CastToCharacter_Player (Components|GetOwner)))
  (bind _output_get (Variables|References|SetAs%20PLAYER _ascharacter_player))
  (Utilities|FlowControl|DelayUntilNextTick)
  (Variables|References|SetUI%20Card%20Holder (Variables|/Game/UI/UI_HUD.UI_HUD_C|GetUI_CardHolder (Variables|/Game/Player/Character_Player.Character_Player_C|GetHUD _output_get)))
  (CallFunction|AddMappingContext)
  (CallFunction|LoadDeck)
  (if (Variables|Default|GetisHandPreFilled)
    (CallFunction|LoadAllCards)
    (else
      (CallFunction|AttemptDrawTimer))))

(event EventTick
  (params (DeltaSeconds :type Float%20%28single-precision%29))
  ;[0 0.6773 1] DEBUG TICk
)

(event Input|KeyboardEvents|DebugKeyC
  (params (Key :type Key%20Structure :default "None") (ActionValue :type Input%20Action%20Value%20Structure))
  (bind (_isblackjack _highcount _lowcount) (CallFunction|CheckforBlackjack))
  ;[0 0.6773 1] DEBUG TICk
  (:Pressed
    (Utilities|FlowControl|FlipFlop
      (:A
        (Utilities|FlowControl|Gate true) ; enters at Open
      )
      (:B
        (Utilities|FlowControl|Gate true) ; enters at Close
      ))))

(fn CheckforBlackjack
  (LocalVariables|SetCurrentTotalLow 0)
  (LocalVariables|SetCurrentTotalHigh 0)
  (for _array_element (Variables|Default|GetHandIDs)
    (bind (_isvalidid _outcardinfo) (CallFunction|GetDatafromID _array_element))
    (if _isvalidid
      (LocalVariables|SetCurrentTotalLow (+ (LocalVariables|GetCurrentTotalLow) (Math|Integer|SelectInt 10 (.Value (Utilities|Struct|BreaksCardInfo _outcardinfo)) (>= (.Value (Utilities|Struct|BreaksCardInfo _outcardinfo)) 10))))
      (LocalVariables|SetCurrentTotalHigh (+ (LocalVariables|GetCurrentTotalHigh) (Math|Integer|SelectInt 11 (Math|Integer|SelectInt 10 (.Value (Utilities|Struct|BreaksCardInfo _outcardinfo)) (>= (.Value (Utilities|Struct|BreaksCardInfo _outcardinfo)) 10)) (== (.Value (Utilities|Struct|BreaksCardInfo _outcardinfo)) 1))))))
  (return (and (or (== (LocalVariables|GetCurrentTotalLow) 21) (== (LocalVariables|GetCurrentTotalHigh) 21)) (not (Utilities|Time|IsValidTimerHandle (Variables|Blackjack|GetBlackjackTimerHandle)))) (LocalVariables|GetCurrentTotalHigh) (LocalVariables|GetCurrentTotalLow)))

(fn GetDatafromID
  (params (ID :type Integer))
  (bind _outrownames (DataTable|GetDataTableRowNames "/Game/BLUEPRINTS/Cards/DT_Cards.DT_Cards"))
  (bind _returnvalue (Utilities|GetDataTableRow "/Game/BLUEPRINTS/Cards/DT_Cards.DT_Cards" (Utilities|Array|Get(acopy) _outrownames (- ID 1)))
    (:then
      (return true _returnvalue))
    (:RowNotFound
      (return false ""))))

(fn GetCardSpawnTransform
  (params (DistanceFromPlayer :type Float%20%28double-precision%29))
  (bind _returnvalue (Components|GetOwner))
  (bind _ascharacter_player (Utilities|Casting|CastToCharacter_Player _returnvalue))
  (bind _returnvalue_2 (Transformation|GetActorLocation _ascharacter_player))
  (bind _returnvalue_3 (Transformation|GetActorForwardVector _ascharacter_player))
  (bind _hitlocation (CallFunction|LineTrace _returnvalue_2 _returnvalue_3 DistanceFromPlayer "ForDuration" "(R=1.000000,G=0.000000,B=0.000000,A=1.000000)"))
  (bind (_x _y) (Math|Vector|BreakVector _hitlocation))
  ;[1 1 1] raycasts from the players forward first, once it hits 400 distance it does another raycast downwards to make sure its on the floor and not in the air
  (return (Math|Transform|MakeTransform (.HitLocation (CallFunction|LineTrace (Math|Vector|MakeVector _x _y 1e+03) "0.000000,0.000000,-1.000000" 1e+04 "ForDuration" "(R=0.000000,G=0.148792,B=1.000000,A=1.000000)")))))

(fn UseCard
  (params (Position :type Integer))
  (bind _output_get (LocalVariables|SetCardID (Utilities|Array|Get(acopy) (Variables|Default|GetHandIDs) Position)))
  (if (== _output_get -1)
    (return false)
    (else
      (bind _isvalidid (CallFunction|GetDatafromID (LocalVariables|GetCardID)))
      (if _isvalidid
        (CallFunction|SpawnCardActor (LocalVariables|GetCardID))
        (Utilities|Array|SetArrayElem (Variables|Default|GetHandIDs) Position -1)
        (Utilities|Array|Add (Variables|Default|GetdiscardPileIDs) (LocalVariables|GetCardID))
        (return true)
        (else
          (return false))))))

(fn GetCardDrawTime
  (return (Math|Float|SelectFloat (Variables|Blackjack|GetBlackjackHandDrawDelay) (Variables|Default|GetCardDrawDelay) (Utilities|Time|IsValidTimerHandle (Variables|Blackjack|GetBlackjackTimerHandle)))))

(fn DiscardHand
  (for (_array_element _array_index) (Variables|Default|GetHandIDs)
    (if (!= _array_element -1)
      (Math|Integer|IncrementInt (LocalVariables|GetcardCount)
        (:%20%20
          (CallFunction|DiscardCard _array_index)))))
  (return (LocalVariables|GetcardCount)))