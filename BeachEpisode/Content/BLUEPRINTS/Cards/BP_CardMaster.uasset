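; BP_CardMaster is a card actor, apparently the base for ability cards, displayed as a coloured cube with a text label.
; Initialise takes a CardInfo, tints the cube by card type and sets the label from its value, showing face cards as 10 plus their letter.
; It then calls ActivateAbility, which starts a one-shot timer of AbilityTime when AbilityTimer is set.
; EndAbility is an empty stub.
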(event Custom|Initialise
  (params (CardInfo :type S%20Card%20Info%20Structure))
  (bind (_value _type) (Utilities|Struct|BreaksCardInfo CardInfo))
  (Rendering|Material|SetVectorParameterValueonMaterials (Variables|Default|GetCube) "Colour" (Math|Conversions|ToVector(LinearColor) (Utilities|Select :Index _type :NewEnumerator0 "(R=0.000000,G=0.286000,B=1.000000,A=1.000000)" :NewEnumerator1 "(R=1.000000,G=0.072917,B=0.072917,A=1.000000)" :NewEnumerator2 "(R=0.145833,G=1.000000,B=0.145833,A=1.000000)" :NewEnumerator3 "(R=0.583333,G=0.583333,B=0.583333,A=1.000000)")))
  (Rendering|Components|TextRender|SetText (Variables|Default|GetTextRender) (Utilities|Select :Index _value :Option%200 "ERROR" :Option%201 "A" :Option%202 "2" :Option%203 "3" :Option%204 "4" :Option%205 "5" :Option%206 "6" :Option%207 "7" :Option%208 "8" :Option%209 "9" :Option%2010 "10" :Option%2011 "10 - J" :Option%2012 "10 - Q" :Option%2013 "10 - K"))
  (CallFunction|ActivateAbility))

(fn ConstructionScript)

(fn ActivateAbility
  (if (Variables|Default|GetAbilityTimer?)
    (Utilities|Time|SetTimerbyEvent (EventDispatchers|CreateEvent :!event EndAbility) (Variables|Default|GetAbilityTime))))

(fn EndAbility)