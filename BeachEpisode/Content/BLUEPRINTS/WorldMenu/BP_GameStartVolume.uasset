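; BP_GameStartVolume walks the player to the game's start point and seals off the Saloon behind them.
; MovePlayer opens a gate on Tick that feeds movement input toward an Arrow component until the player is within a small distance of it.
; On arrival the gate closes, InPosition calls ToggleInputMode to hand control back, and the invisible Wall turns blocking on all channels except Visibility.
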(event Custom|MovePlayer
  (bind _arrow (Variables|Default|GetArrow))
  (bind _as_character_player (Variables|Default|GetAs%20Character%20Player))
  (bind _returnvalue (Transformation|GetWorldLocation _arrow))
  (bind _returnvalue_2 (Transformation|GetActorLocation _as_character_player))
  ;[1 1 1] Moves the player to the start of the game
  (Utilities|FlowControl|Gate true) ; enters at Open
)

(event Custom|InPosition
  (bind _wall (Variables|Default|GetWall))
  ;[1 1 1] Give Player Control Back
  (Default|ToggleInputMode (Variables|Default|GetAs%20Character%20Player) false)
  ;[1 1 1] Make InvisWall so Saloon cant be re-entered
  (Collision|SetCollisionEnabled _wall "QueryAndPhysics")
  (Collision|SetCollisionResponsetoAllChannels _wall "ECR_Block")
  (Collision|SetCollisionResponsetoChannel _wall "ECC_Visibility" "ECR_Ignore"))

(event EventBeginPlay
  (bind _ascharacter_player (Utilities|Casting|CastToCharacter_Player (Game|GetPlayerCharacter 0)))
  (Variables|Default|SetAs%20Character%20Player _ascharacter_player))

(event EventTick
  (params (DeltaSeconds :type Float%20%28single-precision%29))
  (bind _arrow (Variables|Default|GetArrow))
  (bind _as_character_player (Variables|Default|GetAs%20Character%20Player))
  (bind _returnvalue (Transformation|GetWorldLocation _arrow))
  (bind _returnvalue_2 (Transformation|GetActorLocation _as_character_player))
  ;[1 1 1] Moves the player to the start of the game
  (Utilities|FlowControl|Gate true :!label _label
    (:Exit
      (if (> (Math|Vector|Distance(Vector) _returnvalue _returnvalue_2) 5e+01)
        (Pawn|Input|AddMovementInput _as_character_player (Math|Vector|Normalize (Math|Vector|GetUnitDirection(Vector) _returnvalue_2 _returnvalue)) 1.0 false)
        (else
          (Utilities|FlowControl|Sequence
            (:then_0
              (goto _label Close))
            (:then_1
              (CallFunction|InPosition))))))))

(fn ConstructionScript)