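; Weapon pickup that attaches to the hand of the first player to overlap it, adding its input mapping and ammo HUD until dropped.
; Holding shoot fires immediately, then repeats on a looping timer at the WeaponData rate, spending ammo until release or empty.
; Each shot traces from the camera to find the aim point, then from the character toward it so obstacles block fire.
; Hit results are returned but not yet used.
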(event OnComponentBeginOverlap(Sphere)
  (params (OverlappedComponent :type Primitive%20Component%20Object%20Reference) (OtherActor :type Actor%20Object%20Reference) (OtherComp :type Primitive%20Component%20Object%20Reference) (OtherBodyIndex :type Integer) (bFromSweep :type Boolean) (SweepResult :type Hit%20Result%20Structure%20%28by%20ref%29))
  ;[1 1 1] Initial Interaction & Create Refs
  (bind _as_player (Utilities|Casting|CastTo_PLAYER OtherActor))
  (Variables|Default|GetOwningCharacter
    (:then)
    (:else
      (bind _output_get (Variables|Default|SetOwningCharacter _as_player))
      (CallFunction|PickUp _output_get))))

(event Custom|PickUp
  (params (OwningCharacter :type PLAYER%20Object%20Reference))
  (bind _owningcontroller (Variables|/Game/PLAYER/_PLAYER._PLAYER_C|GetOwningController OwningCharacter))
  ;[1 1 1] Attach & Bind to Character
  (Input|AddMappingContext (PlayerController|LocalPlayerSubsystems|GetEnhancedInputLocalPlayerSubsystem _owningcontroller) "/Game/INPUT/IMC_Weapon.IMC_Weapon" 0 "(bIgnoreAllPressedKeysUntilRelease=True,bForceImmediately=False)")
  (Transformation|AttachComponentToComponent (Variables|/Game/PLAYER/_PLAYER._PLAYER_C|GetHandLoc OwningCharacter) "None" "SnapToTarget" "KeepWorld" "KeepWorld" true)
  (Input|EnableInput _owningcontroller)
  (CallFunction|UpdateAmmoHUD true))

(event Custom|Drop
  ;[1 1 1] Detach & Unbind from Character
  (CallFunction|StopShoot)
  (CallFunction|UpdateAmmoHUD false)
  (Transformation|DetachFromActor "KeepWorld" "KeepWorld" "KeepWorld")
  (Input|DisableInput (Variables|/Game/PLAYER/_PLAYER._PLAYER_C|GetOwningController (Variables|Default|GetOwningCharacter)))
  (Input|RemoveMappingContext (PlayerController|LocalPlayerSubsystems|GetEnhancedInputLocalPlayerSubsystem (Variables|/Game/PLAYER/_PLAYER._PLAYER_C|GetOwningController (Variables|Default|GetOwningCharacter))) "/Game/INPUT/IMC_Weapon.IMC_Weapon" "(bIgnoreAllPressedKeysUntilRelease=True,bForceImmediately=False)")
  (Variables|Default|SetOwningCharacter 0))

(event Custom|BeginShoot
  (bind _loadedammo (Variables|Default|GetLoadedAmmo))
  (bind _returnvalue (Utilities|Time|SetTimerbyEvent (delegate Custom|Fire) (Utilities|Struct|BreaksWeaponData (Variables|Default|GetWeaponData)) true))
  (if (>= _loadedammo 1)
    (Math|Integer|DecrementInt _loadedammo
      (:%20%20
        (CallFunction|UpdateAmmoHUD true)
        (CallFunction|AngleAdjustedHitScan)))
    (else
      (Utilities|Time|ClearandInvalidateTimerbyHandle _returnvalue))))

(event Custom|Fire
  (bind _loadedammo (Variables|Default|GetLoadedAmmo))
  (if (>= _loadedammo 1)
    (Math|Integer|DecrementInt _loadedammo
      (:%20%20
        (CallFunction|UpdateAmmoHUD true)
        (CallFunction|AngleAdjustedHitScan)))
    (else
      (Utilities|Time|ClearandInvalidateTimerbyHandle (stale Custom|BeginShoot _returnvalue)))))

(event Custom|StopShoot
  (Utilities|Time|ClearandInvalidateTimerbyHandle (stale Custom|BeginShoot _returnvalue)))

(event Custom|UpdateAmmoHUD
  (params (isVisible :type Boolean))
  (bind _owningcharacter (Variables|Default|GetOwningCharacter)
    (:then
      (Default|UpdateAmmo (Variables|/Game/PLAYER/_PLAYER._PLAYER_C|GetHUD _owningcharacter) isVisible (Variables|Default|GetLoadedAmmo) (Utilities|Struct|BreaksWeaponData (Variables|Default|GetWeaponData))))
    (:else)))

(event Input|EnhancedActionEvents|EnhancedInputActionIA_Drop
  (params (ActionValue :type Boolean) (ElapsedSeconds :type Float%20%28double-precision%29) (TriggeredSeconds :type Float%20%28double-precision%29) (InputAction :type Input%20Action%20Object%20Reference :default "/Game/INPUT/Actions/IA_Drop.IA_Drop"))
  ;[1 1 1] Input to Functions
  (:Started
    (Variables|Default|GetOwningCharacter
      (:then
        (CallFunction|Drop))
      (:else))))

(event Input|EnhancedActionEvents|EnhancedInputActionIA_Reload
  (params (ActionValue :type Boolean) (ElapsedSeconds :type Float%20%28double-precision%29) (TriggeredSeconds :type Float%20%28double-precision%29) (InputAction :type Input%20Action%20Object%20Reference :default "/Game/INPUT/Actions/IA_Reload.IA_Reload"))
  ;[1 1 1] Input to Functions
)

(event Input|EnhancedActionEvents|EnhancedInputActionIA_Shoot
  (params (ActionValue :type Boolean) (ElapsedSeconds :type Float%20%28double-precision%29) (TriggeredSeconds :type Float%20%28double-precision%29) (InputAction :type Input%20Action%20Object%20Reference :default "/Game/INPUT/Actions/IA_Shoot.IA_Shoot"))
  ;[1 1 1] Input to Functions
  (:Started
    (Variables|Default|GetOwningCharacter
      (:then
        (CallFunction|BeginShoot))
      (:else)))
  (:Canceled
    (Variables|Default|GetOwningCharacter :!label _label
      (:then
        (CallFunction|StopShoot))
      (:else)))
  (:Completed
    (goto _label)))

(fn ConstructionScript)

(fn AngleAdjustedHitScan
  (bind _owningcharacter (Variables|Default|GetOwningCharacter))
  (bind _owningcharacter_2 (Variables|Default|GetOwningCharacter))
  (bind _returnvalue (Transformation|GetActorLocation _owningcharacter_2))
  (bind _followcamera (Variables|/Game/PLAYER/_PLAYER._PLAYER_C|GetFollowCamera _owningcharacter))
  ;[1 1 1] Fires two line traces, first from the camera to determine where the middle of the screen collides, then another from the gun to the hit location, so if something is in front of the player and not the camera you cant shoot through it
  (bind _hitlocation (CallFunction|LineTrace (Transformation|GetWorldLocation _followcamera) (Math|Vector|GetForwardVector _followcamera) 1e+04 "ForDuration"))
  (bind (_outhit _returnvalue_2) (Collision|LineTraceByChannel _returnvalue (Utilities|ExtendVector _returnvalue _hitlocation (Utilities|Struct|BreaksWeaponData (Variables|Default|GetWeaponData))) "TraceTypeQuery1" false 0 "ForDuration"))
  (if _returnvalue_2
    (return (.bBlockingHit (Collision|BreakHitResult _outhit)) (.HitActor (Collision|BreakHitResult _outhit)) (.HitComponent (Collision|BreakHitResult _outhit)) (.Location (Collision|BreakHitResult _outhit)))
    (else
      (return false 0 0 (.TraceEnd (Collision|BreakHitResult _outhit))))))