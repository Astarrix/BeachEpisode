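; BP_EnemyController is an enemy AI controller that feeds player perception into the Blackboard.
; Sighting a Character_Player sets CanSeePlayer and PlayerTarget, while losing it starts a PerceptionMaxAge timer, apparently bound to ForgetTarget, which clears both keys.
; Regaining sight does not cancel that timer, so a pending forget can still fire.
; Tick prints the timer's remaining time for debugging.
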(event OnTargetPerceptionUpdated(AIPerception)
  (params (Actor :type Actor%20Object%20Reference) (Stimulus :type AI%20Stimulus%20Structure))
  (bind _returnvalue (Actor|GetComponentbyClass "/Script/AIModule.BlackboardComponent"))
  (if (== (Utilities|GetClass Actor) "/Game/Player/Character_Player.Character_Player_C")
    (if (.bSuccessfullySensed (Utilities|Struct|BreakAIStimulus Stimulus))
      ;[1 1 1] Gained Sight of Player - sets target
      (AI|Components|Blackboard|SetValueasBool _returnvalue (Utilities|String|StringToName "CanSeePlayer") true)
      (AI|Components|Blackboard|SetValueasObject _returnvalue (Utilities|String|StringToName "PlayerTarget") Actor)
      (else
        ;[1 1 1] Lost Sight of Player - starts age timer
        (bind _returnvalue_2 (Utilities|Time|SetTimerbyEvent (EventDispatchers|CreateEvent :!event Custom|ForgetTarget) (Variables|Default|GetperceptionMaxAge)))
        (Variables|Default|SetPerception%20Timer _returnvalue_2)))))

(event Custom|ForgetTarget
  (bind _returnvalue (Actor|GetComponentbyClass "/Script/AIModule.BlackboardComponent"))
  ;[1 1 1] Forgets target when age timer reaches 0
  (AI|Components|Blackboard|SetValueasObject _returnvalue (Utilities|String|StringToName "PlayerTarget") 0)
  (AI|Components|Blackboard|SetValueasBool _returnvalue (Utilities|String|StringToName "CanSeePlayer") false))

(event EventBeginPlay
  (Development|PrintString "Hello" true true "(R=0.000000,G=0.660000,B=1.000000,A=1.000000)" 2.0 "StimAge"))

(event EventTick
  (params (DeltaSeconds :type Float%20%28single-precision%29))
  ;[1 1 1] Perception Age Debug
  (Development|PrintString (Utilities|String|ToString(Float) (Utilities|Time|GetTimerRemainingTimebyHandle (Variables|Default|GetPerception%20Timer))) true true "(R=0.000000,G=0.660000,B=1.000000,A=1.000000)" 2.0 "StimAge"))

(fn ConstructionScript)