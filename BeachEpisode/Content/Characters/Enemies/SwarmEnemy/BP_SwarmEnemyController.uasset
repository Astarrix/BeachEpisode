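; AI controller for the swarm enemy that starts its behavior tree, BT_SwarmEnemy, on BeginPlay.
; It then seeds the Blackboard with the controlled pawn's location as the start position, plus patrol and attack ranges from its own variables.
; The controller graph holds only this one-time setup, done on BeginPlay rather than on possession, with no other logic.
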(event EventBeginPlay
  (bind _returnvalue (AI|GetBlackboard 0))
  (AI|RunBehaviorTree "/Game/Characters/Enemies/SwarmEnemy/BT_SwarmEnemy.BT_SwarmEnemy")
  (AI|Components|Blackboard|SetValueasVector _returnvalue (Utilities|String|StringToName "StartPos") (Transformation|GetActorLocation (Pawn|GetControlledPawn)))
  (AI|Components|Blackboard|SetValueasFloat _returnvalue (Utilities|String|StringToName "PatrolRange") (Variables|Default|GetPatrolRadius))
  (AI|Components|Blackboard|SetValueasFloat _returnvalue (Utilities|String|StringToName "AttackRange") (Variables|Default|GetAttackRange)))

(fn ConstructionScript)