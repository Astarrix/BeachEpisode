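; Spawn effect actor that delays the appearance of a swarm enemy behind a summoning cue.
; BeginPlay plays the DemonSummon sound at world origin, then a one-shot timer removes the Sphere component and spawns the enemy just above the actor, rotated toward the player.
; The Type select currently maps every option to BP_SwarmEnemy.
; A debug print shows the spawn rotation; the spawn validity check is disconnected, and the effect actor is never destroyed here.
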(event Custom|Spawn%20Enemy
  (bind _returnvalue (Game|Player|GetPlayerPawn 0))
  (bind _returnvalue_2 (Transformation|GetActorLocation))
  (bind _returnvalue_3 (Transformation|GetActorLocation _returnvalue))
  (bind _returnvalue_4 (Math|Rotator|FindLookatRotation _returnvalue_2 _returnvalue_3))
  (Development|PrintString (Utilities|String|ToString(Rotator) _returnvalue_4))
  (Components|DestroyComponent (Variables|Default|GetSphere))
  (bind _returnvalue_5 (Game|SpawnActorfromClass (Utilities|Select :Index (Variables|Default|GetType) :NewEnumerator1 "/Game/Characters/Enemies/SwarmEnemy/BP_SwarmEnemy.BP_SwarmEnemy_C" :NewEnumerator0 "/Game/Characters/Enemies/SwarmEnemy/BP_SwarmEnemy.BP_SwarmEnemy_C" :NewEnumerator2 "/Game/Characters/Enemies/SwarmEnemy/BP_SwarmEnemy.BP_SwarmEnemy_C") (Math|Transform|MakeTransform (+ (Transformation|GetActorLocation) "0.000000,0.000000,50.000000") _returnvalue_4) "Undefined" "MultiplyWithRoot" 0 0)))

(event EventBeginPlay
  (Audio|PlaySoundatLocation "/Game/Characters/Enemies/EnemySpawner/Particles/Assets/DemonSummon.DemonSummon" "0, 0, 0" "0, 0, 0" 1.0 1.0 0.0 0 0 0 0)
  (Utilities|Time|SetTimerbyEvent (delegate Custom|Spawn%20Enemy) 1.5))

(fn ConstructionScript)