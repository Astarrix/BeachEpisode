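; Damageable enemy spawner that spawns enemies while the player stays within its trigger radius.
; Overlap triggers an immediate attempt and a looping timer with a once-randomised interval, cleared when an attempt finds the player out of range.
; Each attempt picks an under-cap type from a weighted array and spawns BP_EnemySpawnEffect at a random reachable nearby point.
; BPHealthComponent takes damage; a timeline animates the health widget, turning the cube red at zero.
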(event OnComponentBeginOverlap(Sphere)
  (params (OverlappedComponent :type Primitive%20Component%20Object%20Reference) (OtherActor :type Actor%20Object%20Reference) (OtherComp :type Primitive%20Component%20Object%20Reference) (OtherBodyIndex :type Integer) (bFromSweep :type Boolean) (SweepResult :type Hit%20Result%20Structure%20%28by%20ref%29))
  ;[1 1 1] OnColliderEnter
  (if (and (== OtherActor (Variables|Default|GetPlayer)) (not (Utilities|Time|IsTimerActivebyHandle (Variables|Default|GetSpawnTimer))))
    (CallFunction|AttemptSpawnEnemy)
    (bind _returnvalue (Utilities|Time|SetTimerbyEvent (EventDispatchers|CreateEvent :!event Custom|AttemptSpawnEnemy) (CallFunction|CreateRandomisedTimerLength) true))
    (Variables|Default|SetSpawnTimer _returnvalue)))

(event Custom|AttemptSpawnEnemy
  (if (CallFunction|IsPlayerWithinSpawnRange?)
    (bind _type_found (CallFunction|CheckifEnemyCanSpawn))
    (if (Utilities|Enum|Equal(Enum) _type_found "NewEnumerator1")
      (Development|PrintString "MaxEnemies")
      (else
        ;[1 1 1] Increments currentSpawned in Struct Array
        ;;[1 1 1] Length based ForLoop because a ForLoop gets a copy and not a modifyable ref
        (for _index (range 0 (- (Utilities|Array|Length (Variables|Default|GetSpawnableEnemies)) 1))
          (if (Utilities|Enum|Equal(Enum) _type_found (.Type (Utilities|Struct|BreakS_EnemySpawn (Utilities|Array|Get(acopy) (Variables|Default|GetSpawnableEnemies) _index))))
            (bind _result (Math|Integer|IncrementInt (.CurrentlySpawned (Utilities|Struct|BreakS_EnemySpawn (Utilities|Array|Get(acopy) (Variables|Default|GetSpawnableEnemies) _index))))
              (:%20%20
                (Game|SpawnActorfromClass "/Game/Characters/Enemies/EnemySpawner/Particles/BP_EnemySpawnEffect.BP_EnemySpawnEffect_C" (Math|Transform|MakeTransform (.RandomLocation (AI|Navigation|GetRandomReachablePointinRadius (Transformation|GetActorLocation) (Variables|Default|GetSpawnRange) 0 0))) "Undefined" "MultiplyWithRoot" 0 _type_found self 0)))))))
    (else
      (Utilities|Time|ClearandInvalidateTimerbyHandle (Variables|Default|GetSpawnTimer)))))

(event Custom|AddProbabilities
  ;[1 1 1] Init
  ;;[1 1 1] Setup enemy probabilities
  (for _array_element (Variables|Default|GetSpawnableEnemies)
    (for _index (range 1 (.ProbabilityWeight (Utilities|Struct|BreakS_EnemySpawn _array_element)))
      (Utilities|Array|Add (Variables|Default|GetprobabilityChecker) (.Type (Utilities|Struct|BreakS_EnemySpawn _array_element))))))

(event Custom|EnemyDeath
  (params (Enemy%20Type :type E_EnemyType%20Enum :default "NewEnumerator1")))

(event EventInitHealthUI
  (params (MaxHealth :type Float%20%28double-precision%29) (Current%20Health :type Float%20%28double-precision%29))
  (Utilities|FlowControl|DelayUntilNextTick)
  (bind _asw_spatial_health (Utilities|Casting|CastToW_SpatialHealth (UserInterface|GetWidget (Variables|Default|GetWidget))))
  (bind _output_get (Variables|Default|SetSpatial%20Health%20Widget _asw_spatial_health))
  (Default|SetHealth _output_get (/ MaxHealth Current%20Health)))

(event EventUpdateHealthUI
  (params (NewHealth :type Float%20%28double-precision%29) (MaxHealth :type Float%20%28double-precision%29))
  (Variables|Default|SethealthAnimStart (Variables|/Script/UMG.ProgressBar|GetPercent (Variables|/Game/Characters/Enemies/W_SpatialHealth.W_SpatialHealth_C|GetHealthBar (Variables|Default|GetSpatial%20Health%20Widget))))
  (Variables|Default|SethealthAnimEnd (/ NewHealth MaxHealth))
  (bind _alpha (Timeline|Timeline PlayFromStart)
    (:Update
      (Default|SetHealth (Variables|Default|GetSpatial%20Health%20Widget) (Math|Float|Lerp (Variables|Default|GethealthAnimStart) (Variables|Default|GethealthAnimEnd) _alpha)))
    (:Finished
      (if (== (Variables|/Game/Characters/BP_HealthComponent.BP_HealthComponent_C|GetCurrentHealth (Variables|Default|GetBP_HealthComponent)) 0.0)
        (Rendering|Material|SetMaterial (Variables|Default|GetCube) 0 "/Game/Characters/Enemies/SwarmEnemy/SwarmChildren/M_Red.M_Red")))))

(event EventBeginPlay
  ;[1 1 1] Init
  (bind _asbp_character_player (Utilities|Casting|CastToBP_Character_Player (Game|Player|GetPlayerPawn 0)))
  (Variables|Default|SetPlayer _asbp_character_player)
  (Variables|Default|SetSpawnDelayOnAggro (* (Variables|Default|GetSpawnDelayAverage) 0.5))
  (CallFunction|AddProbabilities))

(event Game|Damage|EventAnyDamage
  (params (Damage :type Float%20%28single-precision%29) (DamageType :type Damage%20Type%20Object%20Reference) (InstigatedBy :type Controller%20Object%20Reference) (DamageCauser :type Actor%20Object%20Reference))
  (Default|TakeDamage (Variables|Default|GetBP_HealthComponent) Damage))

(fn ConstructionScript
  (Components|Sphere|SetSphereRadius (Variables|Default|GetSphere) (Variables|Default|GetPlayerSpawnTriggerDistance) true))

(fn CheckifEnemyCanSpawn
  (LocalVariables|SettempProbabilityChecker (Variables|Default|GetprobabilityChecker))
  (while (!= (Utilities|Array|Length (LocalVariables|GettempProbabilityChecker)) 0)
    (LocalVariables|SetenemyTypeToCheck (.OutItem (Utilities|Array|Random (LocalVariables|GettempProbabilityChecker))))
    (for _array_element (Variables|Default|GetSpawnableEnemies)
      ;[1 1 1 1 12] Is the random enemy of the struct's type?
      (if (Utilities|Enum|Equal(Enum) (.Type (Utilities|Struct|BreakS_EnemySpawn _array_element)) (LocalVariables|GetenemyTypeToCheck))
        ;[1 1 1 1 14] Is this type at max quantity?
        (if (< (.CurrentlySpawned (Utilities|Struct|BreakS_EnemySpawn _array_element)) (.MaxAmount (Utilities|Struct|BreakS_EnemySpawn _array_element)))
          (LocalVariables|SetenemyFound? (.Type (Utilities|Struct|BreakS_EnemySpawn _array_element)))
          (Utilities|Array|Clear (LocalVariables|GettempProbabilityChecker))
          (else
            (Utilities|Array|RemoveItem (LocalVariables|GettempProbabilityChecker) (LocalVariables|GetenemyTypeToCheck)))))))
  (return (LocalVariables|GetenemyFound?)))

(fn IsPlayerWithinSpawnRange?
  (return (<= (Math|Vector|Distance(Vector) (Transformation|GetActorLocation) (Transformation|GetActorLocation (Variables|Default|GetPlayer))) (+ (Variables|Default|GetPlayerSpawnTriggerDistance) 5e+01))))

(fn CreateRandomisedTimerLength
  (bind _spawndelayaverage (Variables|Default|GetSpawnDelayAverage))
  (return (Math|Random|RandomFloatinRange (* _spawndelayaverage 0.75) (* _spawndelayaverage 1.25))))