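; BP_HealthComponent is a health component that tracks its owner's health and destroys the owning actor when health runs out.
; Health starts at MaxHealth on BeginPlay, and TakeDamage subtracts from it and prints the remainder while CanTakeDamage is true.
; At zero or below it calls Die, then turns CanTakeDamage off for IframeDuration, so that invulnerability window follows only a lethal hit.
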(event Custom|TakeDamage
  (params (Damage :type Float%20%28double-precision%29))
  (if (Variables|Default|GetCanTakeDamage)
    (bind _output_get (Variables|Default|SetCurrentHealth (- (Variables|Default|GetCurrentHealth) Damage)))
    (Development|PrintString (Utilities|String|Append "Health Remaining - " (Utilities|String|ToString(Float) _output_get)))
    (if (<= _output_get 0.0)
      (CallFunction|Die)
      (Variables|Default|SetCanTakeDamage false)
      (Utilities|FlowControl|Delay (Variables|Default|Geti-frameDuration))
      (Variables|Default|SetCanTakeDamage true))))

(event Custom|Die
  (Actor|DestroyActor (Components|GetOwner)))

(event EventBeginPlay
  (Variables|Default|SetCurrentHealth (Variables|Default|GetMaxHealth)))

(event EventTick
  (params (DeltaSeconds :type Float%20%28single-precision%29)))