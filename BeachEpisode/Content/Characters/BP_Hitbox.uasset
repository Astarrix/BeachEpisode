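; BP_Hitbox is a short-lived attack hitbox actor that damages opposing-team characters it touches.
; On overlap, its Box checks for BPI_Characters and compares IsEnemy against the target's health component before applying damage.
; If CausesStun is set and the target implements BPI_Stun, it sends a stun message.
; It destroys itself after that first valid hit, or when its LifeSpan delay runs out.
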(event OnComponentBeginOverlap(Box)
  (params (OverlappedComponent :type Primitive%20Component%20Object%20Reference) (OtherActor :type Actor%20Object%20Reference) (OtherComp :type Primitive%20Component%20Object%20Reference) (OtherBodyIndex :type Integer) (bFromSweep :type Boolean) (SweepResult :type Hit%20Result%20Structure%20%28by%20ref%29))
  (if (Utilities|DoesObjectImplementInterface OtherActor "/Game/Characters/Enemies/BPI_Characters.BPI_Characters_C")
    (if (!= (Variables|Default|GetIsEnemy) (Variables|/Game/Characters/BP_HealthComponent.BP_HealthComponent_C|GetIsEnemy (Actor|GetComponentbyClass OtherActor "/Game/Characters/BP_HealthComponent.BP_HealthComponent_C")))
      (Game|Damage|ApplyDamage OtherActor (Variables|Default|GetDamage) 0 0)
      (if (and (Utilities|DoesObjectImplementInterface OtherActor "/Game/Characters/Enemies/BPI_Stun.BPI_Stun_C") (Variables|Default|GetCausesStun))
        (Class|BPIStun|Stun(Message) OtherActor))
      (Actor|DestroyActor))))

(event EventBeginPlay
  (Utilities|FlowControl|Delay (Variables|Default|GetLifeSpan))
  (Actor|DestroyActor))

(event Collision|EventActorBeginOverlap
  (params (OtherActor :type Actor%20Object%20Reference)))

(event EventTick
  (params (DeltaSeconds :type Float%20%28single-precision%29)))

(fn ConstructionScript)